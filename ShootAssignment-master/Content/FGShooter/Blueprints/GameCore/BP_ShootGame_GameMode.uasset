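; Game mode for the shooter game that plays the theme music on begin play and handles enemy tracking and the win condition.
; RegisterEnemyDeath removes enemies from the BPEnemy array, and CheckEnemies calls WinGame on the game state once that array is empty.
; Helper functions increment the current wave counter and spawn spider enemies at a given target point's transform.
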(event Custom|CheckEnemies
  ;[0.6291 0.6795 1] Check if player have defeated all the spawning enemy waves (current setting 3). If player is the last standing man, show win game.
  (if (== (Utilities|Array|Length (Variables|Default|GetBP_Enemy)) 0)
    (bind _asbp_shoot_game_game_state (Utilities|Casting|CastToBP_ShootGame_GameState (Game|GetGameState)))
    (Default|WinGame _asbp_shoot_game_game_state)))

(event EventBeginPlay
  ;[0.5541 0.6092 1] Play theme music
  (Audio|PlaySound2D "/Game/Sounds/Music/ShooterGame_Music_Cue.ShooterGame_Music_Cue" 1.0 1.0 0.0 0 0))

(fn ConstructionScript)

(fn SetUpNewWave
  (Math|Integer|IncrementInt (Variables|SpawnWave|GetCurrentWave)))

(fn RegisterEnemyDeath
  (params (Enemy :type BP%20Enemy%20Base%20Object%20Reference%20%28by%20ref%29))
  (Utilities|Array|RemoveItem (Variables|Default|GetBP_Enemy) Enemy))

(fn SpawnSpiderfromTargetPoint
  (params (TargetPoint :type Target%20Point%20Object%20Reference))
  (Game|SpawnActorfromClass "/Game/FGShooter/Blueprints/Actor/AI/Spider/BPChild_EnemySpider.BPChild_EnemySpider_C" (Transformation|GetActorTransform TargetPoint) "Undefined" 0 0))