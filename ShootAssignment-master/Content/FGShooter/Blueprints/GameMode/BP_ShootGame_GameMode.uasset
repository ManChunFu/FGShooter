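; BP_ShootGame_GameMode is the shooter's game mode, tracking enemies, a wave counter and the win condition.
; RegisterEnemyDeath removes an enemy from the BPEnemy array.
; CheckEnemies, a separate event not called within this Blueprint, calls WinGame on BP_ShootGame_GameState when that array is empty.
; SetUpNewWave only increments CurrentWave, with no spawning or link to the win check.
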(event Custom|CheckEnemies
  (if (== (Utilities|Array|Length (Variables|Default|GetBP_Enemy)) 0)
    (bind _asbp_shoot_game_game_state (Utilities|Casting|CastToBP_ShootGame_GameState (Game|GetGameState)))
    (Default|WinGame _asbp_shoot_game_game_state)))

(fn ConstructionScript)

(fn SetUpNewWave
  (Math|Integer|IncrementInt (Variables|Default|GetCurrentWave)))

(fn RegisterEnemyDeath
  (params (Enemy :type BP%20Enemy%20Base%20Object%20Reference%20%28by%20ref%29))
  (Utilities|Array|RemoveItem (Variables|Default|GetBP_Enemy) Enemy))