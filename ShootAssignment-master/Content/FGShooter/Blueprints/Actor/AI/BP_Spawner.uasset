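; BP_Spawner is an actor that spawns batches of AI enemies at its Arrow component's location and rotation.
; Its Spawn event uses the class, behavior tree and count from the passed SpawnData, falling back to the spawner's own defaults when that class is invalid.
; Each spawned BP_EnemyBase is added to the BPEnemy array on BP_ShootGame_GameMode.
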(event EventSpawn
  (params (SpawnData :type F%20Spawn%20Data%20Structure))
  (bind (_class _behaviortree _numtospawn) (Utilities|Struct|BreakFSpawnData SpawnData))
  (bind _arrow (Variables|Default|GetArrow))
  (bind _returnvalue (Utilities|IsValidClass _class))
  (for _index (range 0 (- (select _returnvalue _numtospawn (Variables|Default|GetNumToSpawn)) 1))
    (bind _returnvalue_2 (AI|SpawnAIFromClass (select _returnvalue _class (Variables|Default|GetSpawnClass)) (select _returnvalue _behaviortree (Variables|Default|GetSpawnBehaviorTree)) (Transformation|GetWorldLocation _arrow) (Transformation|GetWorldRotation _arrow) false))
    (Utilities|IsValid _returnvalue_2
      (:Is%20Valid
        (bind _asbp_enemy_base (Utilities|Casting|CastToBP_EnemyBase _returnvalue_2))
        (bind _asbp_shoot_game_game_mode (Utilities|Casting|CastToBP_ShootGame_GameMode (Game|GetGameMode)))
        (Utilities|Array|Add (Variables|/Game/FGShooter/Blueprints/GameMode/BP_ShootGame_GameMode.BP_ShootGame_GameMode_C|GetBP_Enemy _asbp_shoot_game_game_mode) _asbp_enemy_base)))))

(fn ConstructionScript)