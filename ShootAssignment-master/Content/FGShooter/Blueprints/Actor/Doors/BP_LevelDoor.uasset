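; BP_LevelDoor is a key card door actor that slides open when a player carrying the card enters its overlap area.
; On BeginPlay it adds a WBP_LevelDoor widget holding a door reference, intended to show info to a nearby player lacking the card.
; Overlaps set the proximity and key card flags.
; The DoorMoveUp timeline drives the door's relative Z, with a Delay on its Update pin triggering the reverse.
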(event EventBeginPlay
  ;[0.6012 0.6727 1] Create level door info on the screen with hidden default setting.
  (bind _returnvalue (UserInterface|CreateWidget "/Game/FGShooter/UI/WBP_LevelDoor.WBP_LevelDoor_C" 0 self))
  (UserInterface|Viewport|AddtoViewport _returnvalue 0))

(event Collision|EventActorBeginOverlap
  (params (OtherActor :type Actor%20Object%20Reference))
  ;[0.604 0.6394 1] If player is near the door AND doesn't have key card then show the info. Hide the info when player is away. Open the door if player has key card.
  (Utilities|IsPlayer OtherActor
    (:IsPlayer
      (Variables|Default|SetIsPlayerNear true)
      (bind _asfirst_person (Utilities|Casting|CastToFirstPerson (Game|Player|GetPlayerPawn 0)))
      (if (Variables|/Game/FGShooter/Blueprints/FirstPerson.FirstPerson_C|GetKeyCard _asfirst_person)
        (Variables|Default|SetHasKeyCard true)
        (bind _dooropen (Timeline|DoorMoveUp Play)
          (:Update
            (Transformation|SetRelativeLocation (Variables|Default|GetDoor) (Math|Vector|MakeVector 0.0 0.0 _dooropen) false false)
            (Utilities|FlowControl|Delay 5.0)
            (Timeline|DoorMoveUp Reverse)))))))

(event Collision|EventActorEndOverlap
  (params (OtherActor :type Actor%20Object%20Reference))
  ;[0.604 0.6394 1] If player is near the door AND doesn't have key card then show the info. Hide the info when player is away. Open the door if player has key card.
  (Variables|Default|SetIsPlayerNear false))

(fn ConstructionScript)